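; Trigger actor that opens a UI_Typing text-entry widget when something overlaps its box, apparently a prototype for in-game keyboard typing.
; The overlap adds the widget, focuses it in Game-and-UI input mode and shows the cursor, which the Show Mouse action also does.
; Debug key events print input, with F and G enabling and disabling actor input.
; CloseUI restores game-only input and clears KeyboardEnable without removing the widget.
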(event `self.ReceiveBeginPlay`)

(event `self.ReceiveActorBeginOverlap`
  (params (OtherActor :type "Actor Object Reference")))

(event `self.Box_Trigger.OnComponentBeginOverlap`
  (params (OverlappedComponent :type "PrimitiveComponent Object Reference") (OtherActor :type "Actor Object Reference") (OtherComp :type "PrimitiveComponent Object Reference") (OtherBodyIndex :type Integer) (bFromSweep :type Boolean) (SweepResult :type "HitResult Structure (by ref)"))
  (bind _returnvalue (`GameplayStatics.GetPlayerController` 0))
  ;[1 1 1] When Player Activates Trigger Show the UI
  (set `self.Box_Trigger` (`self.Box_Trigger`))
  (`KismetSystemLibrary.PrintString` "Trigger Keyboar Activated")
  (bind _returnvalue_2 (`|CreateWidget` "/Game/UI/UI_Typing.UI_Typing_C"))
  (bind _output_get (set `self.UI_Input_Text` _returnvalue_2))
  (set `self.Keyboard Enable` true)
  (`UserWidget.AddToViewport` _output_get 0)
  (`WidgetBlueprintLibrary.SetInputMode_GameAndUIEx` _returnvalue (`self.UI_Input_Text`))
  (`GameplayStatics.SetViewportMouseCaptureMode` "NoCapture")
  (set `PlayerController.bShowMouseCursor` true _returnvalue :!label _label))

(event `InputAction|Show Mouse`
  (params (Key :type "Key Structure"))
  ;[1 1 1] When Player Activates Trigger Show the UI
  (:`Pressed`
    (goto _label)))

(event `self.Box_Trigger.OnComponentEndOverlap`
  (params (OverlappedComponent :type "PrimitiveComponent Object Reference") (OtherActor :type "Actor Object Reference") (OtherComp :type "PrimitiveComponent Object Reference") (OtherBodyIndex :type Integer)))

(event `Key|AnyKey`
  (params (Key :type "Key Structure"))
  ;[1 1 1] Check for Keyboard Input
  (:`Pressed`
    (bind _output_get (set `self.Key` Key))
    (`KismetSystemLibrary.PrintText` (`KismetTextLibrary.Conv_BoolToText` (`KismetInputLibrary.Key_IsKeyboardKey` _output_get)))
    (`KismetSystemLibrary.PrintString` "Hello")))

(event `Key|W`
  (params (Key :type "Key Structure"))
  ;[1 1 1] Check for Keyboard Input
  (:`Pressed`
    (`KismetSystemLibrary.PrintString` "W Key")))

(event `Key|A`
  (params (Key :type "Key Structure"))
  ;[1 1 1] Check for Keyboard Input
)

(event `Key|F`
  (params (Key :type "Key Structure"))
  (:`Pressed`
    (`KismetSystemLibrary.PrintString` "F Enable Input")
    (set `self.Keyboard Enable` true)
    (`self.EnableInput` (`GameplayStatics.GetPlayerController` 0)) ; Get Player Controller Actor
    (`KismetSystemLibrary.PrintText` "Keyboard BP Activated")))

(event `Key|G`
  (params (Key :type "Key Structure"))
  (:`Pressed`
    (`self.DisableInput` null)
    (`KismetSystemLibrary.PrintString` "Keyboard disabled")))

(fn `Close UI`
  (`WidgetBlueprintLibrary.SetInputMode_GameOnly` (`GameplayStatics.GetPlayerController` 0))
  (set `self.Keyboard Enable` false))

(fn `UserConstructionScript`)