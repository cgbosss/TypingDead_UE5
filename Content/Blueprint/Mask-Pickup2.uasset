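; Mask pickup actor that registers itself with the first-person character when its trigger volume is overlapped.
; On overlap begin it finds every BP_FirstPersonCharacter, calls MaskEquipOn, sets TempMaskVar to its MaskSelf variable and calls AddMaskToArrayInv.
; On overlap end it calls MaskEquipOff on the cached character reference.
; The overlapping actor is never checked, and the debug print chains are disconnected.
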(event `self.PickupTrigger.OnComponentBeginOverlap`
  (params (OverlappedComponent :type "PrimitiveComponent Object Reference") (OtherActor :type "Actor Object Reference") (OtherComp :type "PrimitiveComponent Object Reference") (OtherBodyIndex :type Integer) (bFromSweep :type Boolean) (SweepResult :type "HitResult Structure (by ref)"))
  (bind _first_person_ref (`self.First Person Ref`))
  (bind _outactors (`GameplayStatics.GetAllActorsOfClass` "/Game/FirstPerson/Blueprints/BP_FirstPersonCharacter.BP_FirstPersonCharacter_C"))
  (bind _output_get (set `self.Out Actors` _outactors))
  (for _array_element _output_get
    (bind _output_get_2 (set `self.First Person Ref` _array_element))
    (`/Game/FirstPerson/Blueprints/BP_FirstPersonCharacter.Mask Equip On` _output_get_2)
    (set `/Game/FirstPerson/Blueprints/BP_FirstPersonCharacter.TempMaskVar` (`self.MaskSelf`) _first_person_ref)
    (`/Game/FirstPerson/Blueprints/BP_FirstPersonCharacter.Add Mask to Array Inv` _first_person_ref) ; Add Mask to the Inventory
  ))

(event `self.PickupTrigger.OnComponentEndOverlap`
  (params (OverlappedComponent :type "PrimitiveComponent Object Reference") (OtherActor :type "Actor Object Reference") (OtherComp :type "PrimitiveComponent Object Reference") (OtherBodyIndex :type Integer))
  (`GameplayStatics.GetAllActorsOfClass` "/Game/FirstPerson/Blueprints/BP_FirstPersonCharacter.BP_FirstPersonCharacter_C")
  (`/Game/FirstPerson/Blueprints/BP_FirstPersonCharacter.Mask Equip Off` (`self.First Person Ref`)))

(fn `UserConstructionScript`)