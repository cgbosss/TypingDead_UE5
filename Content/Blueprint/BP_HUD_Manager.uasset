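; HUD manager Blueprint that builds the in-game menu UI at BeginPlay, after setting the player's input to game only.
; It creates the main HUD widget and the in-game settings menu, stores both in a list, then loops over it to add each to the viewport.
; ShowTimer prints game time for debugging, while ShowMenu and the keyboard UI function are unfinished stubs.
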(event `self.ReceiveBeginPlay`
  (bind _gamemenu_widget_list (`self.GameMenu_Widget_List`))
  (`WidgetBlueprintLibrary.SetInputMode_GameOnly` (`GameplayStatics.GetPlayerController` 0))
  (`KismetSystemLibrary.PrintString` "HUD Manager Activated")
  ;[1 1 1] Show the Game Menu Widget
  (bind _returnvalue (`|CreateWidget` (`self.Widget HUD`) (`self.GetOwningPlayerController`)))
  (bind _output_get (set `self.Widget_HUD_var` _returnvalue))
  (`KismetArrayLibrary.Array_Add` (`self.GameMenu_Widget_List`) _output_get)
  ;[1 1 1] Settings Menu Widget
  (bind _returnvalue_2 (`|CreateWidget` "/Game/UI/UI_Game_Menu_InSettings.UI_Game_Menu_InSettings_C" (`self.GetOwningPlayerController`))) ; In Game Settings Menu
  (bind _output_get_2 (set `self.Widget_Menu_Settings_IG` _returnvalue_2))
  (`KismetArrayLibrary.Array_Add` _gamemenu_widget_list _output_get_2)
  (for _array_element _gamemenu_widget_list
    (`KismetSystemLibrary.PrintString` (`KismetSystemLibrary.GetDisplayName` _array_element))
    (`UserWidget.AddToViewport` _array_element 0)))

(event `self.ReceiveActorBeginOverlap`
  (params (OtherActor :type "Actor Object Reference")))

(fn `Show the Keyboard UI`)

(fn `ShowMenu`
  (`KismetSystemLibrary.PrintString` "Show Menu")
  (`|CreateWidget` "/Game/UI/UI_Game_Menu_HUD.UI_Game_Menu_HUD_C"))

(fn `ShowTimer`
  (bind _returnvalue (`KismetSystemLibrary.GetGameTimeInSeconds`))
  (`KismetSystemLibrary.PrintText` "BP Hud Show Time FUnction")
  (`KismetSystemLibrary.PrintString` (`KismetStringLibrary.Conv_DoubleToString` _returnvalue) true true (struct :`G` 0.66 :`B` 1.0 :`A` 1.0) _returnvalue))

(fn `UserConstructionScript`)