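; Mask pickup actor that equips a mask on the first-person character when its PickupTrigger is overlapped.
; Overlap start finds every BP_FirstPersonCharacter in the level and calls MaskEquipOn on each, without checking which actor overlapped or removing the pickup.
; Pickup prompts are only debug prints for showing and hiding icons and text, plus a print of the character's name.
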(event `self.PickupTrigger.OnComponentBeginOverlap`
  (params (OverlappedComponent :type "PrimitiveComponent Object Reference") (OtherActor :type "Actor Object Reference") (OtherComp :type "PrimitiveComponent Object Reference") (OtherBodyIndex :type Integer) (bFromSweep :type Boolean) (SweepResult :type "HitResult Structure (by ref)"))
  (`KismetSystemLibrary.PrintText` "Show Pickup Icons and Text")
  (bind _outactors (`GameplayStatics.GetAllActorsOfClass` "/Game/FirstPerson/Blueprints/BP_FirstPersonCharacter.BP_FirstPersonCharacter_C"))
  (bind _output_get (set `self.Out Actors` _outactors))
  (for _array_element _output_get
    (bind _output_get_2 (set `self.First Person Ref` _array_element))
    (`/Game/FirstPerson/Blueprints/BP_FirstPersonCharacter.Mask Equip On` _output_get_2))
  (`KismetSystemLibrary.PrintString` (`KismetSystemLibrary.GetDisplayName` _array_element)))

(event `self.PickupTrigger.OnComponentEndOverlap`
  (params (OverlappedComponent :type "PrimitiveComponent Object Reference") (OtherActor :type "Actor Object Reference") (OtherComp :type "PrimitiveComponent Object Reference") (OtherBodyIndex :type Integer))
  (`KismetSystemLibrary.PrintString` "Hide Pickup Dialog Text and Icons"))

(fn `UserConstructionScript`)